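; Player character Blueprint that registers the Lazarus Enhanced Input mapping context when play begins.
; BeginPlay calls a helper that casts the controller to a player controller, gets its Enhanced Input local player subsystem and adds the context, printing success or failure messages.
; Input action events for forward, backward, left and right movement exist but are empty, so no movement logic is implemented here yet.
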(event `self.ReceiveBeginPlay`
  (`self.AddPlayerCharacterMappingContext`))

(event `EnhancedInput|/Game/InputActions/ForwardInputAction`
  (params (ActionValue :type Boolean) (ElapsedSeconds :type "Float (double-precision)") (TriggeredSeconds :type "Float (double-precision)") (InputAction :type "InputAction Object Reference" :default "/Game/InputActions/ForwardInputAction.ForwardInputAction")))

(event `EnhancedInput|/Game/InputActions/BackwardInputAction`
  (params (ActionValue :type Boolean) (ElapsedSeconds :type "Float (double-precision)") (TriggeredSeconds :type "Float (double-precision)") (InputAction :type "InputAction Object Reference" :default "/Game/InputActions/BackwardInputAction.BackwardInputAction")))

(event `EnhancedInput|/Game/InputActions/MoveLeft`
  (params (ActionValue :type Boolean) (ElapsedSeconds :type "Float (double-precision)") (TriggeredSeconds :type "Float (double-precision)") (InputAction :type "InputAction Object Reference" :default "/Game/InputActions/MoveLeft.MoveLeft")))

(event `EnhancedInput|/Game/InputActions/MoveRight`
  (params (ActionValue :type Boolean) (ElapsedSeconds :type "Float (double-precision)") (TriggeredSeconds :type "Float (double-precision)") (InputAction :type "InputAction Object Reference" :default "/Game/InputActions/MoveRight.MoveRight")))

(fn `AddPlayerCharacterMappingContext`
  (bind _asplayer_controller (cast `PlayerController` (`self.GetController`))
    (:`then`
      (bind _returnvalue (pcsubsystem `EnhancedInputLocalPlayerSubsystem` _asplayer_controller))
      (`/Engine/EditorBlueprintResources/StandardMacros.IsValid` _returnvalue
        (:`Is Valid`
          (`EnhancedInputSubsystemInterface.AddMappingContext` _returnvalue "/Game/InputContexes/LazarusInputContext.LazarusInputContext" 0 (struct))
          (`KismetSystemLibrary.PrintString` (`KismetTextLibrary.Conv_TextToString` (`|FormatText` "{0} mapped input actions" self)) false))
        (:`Is Not Valid`
          (`KismetSystemLibrary.PrintString` "Error: Could not get enhanced input local subsystem, unable to map input context" true true (struct :`G` 0.66 :`B` 1.0 :`A` 1.0) 11.0))))
    (:`CastFailed`
      (`KismetSystemLibrary.PrintString` "Error: Could not get player controller, unable to map input context" true true (struct :`G` 0.66 :`B` 1.0 :`A` 1.0) 11.0))))

(fn `UserConstructionScript`)