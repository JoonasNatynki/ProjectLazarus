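; Simple spawn volume actor that pairs a box shape with a Spawner component to define where a spawnable can appear.
; The construction script registers SpawnBox with the Spawner and passes on Spawnable if valid; the event graph is empty.
; GetRandomPointInVolumeToGround picks a random point in the box and line-traces down by the Arrow's length on Visibility.
; It returns the hit location without checking for a hit.
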(event `self.ReceiveBeginPlay`)

(fn `GetRandomPointInVolumeToGround`
  (returns (Location :type "Vector Structure"))
  (bind _returnvalue (`E4CodeHelpers.FindRandomPointInsideShapeComponent` (`self.SpawnBox`)))
  (bind _outhit (`KismetSystemLibrary.LineTraceSingle` _returnvalue (+ _returnvalue (`KismetMathLibrary.MakeVector` 0.0 0.0 (* (`ArrowComponent.ArrowLength` (`self.Arrow`)) -1.0))) "TraceTypeQuery1" true))
  (return (`.Location` (`GameplayStatics.BreakHitResult` _outhit))))

(fn `UserConstructionScript`
  (`SpawnerComponent.AddSpawnableShape` (`self.Spawner`) (`self.SpawnBox`))
  (bind _spawnable (`self.Spawnable`)
    (:`then`
      (`SpawnerComponent.SetSpawnable` (`self.Spawner`) _spawnable))
    (:`else`)))