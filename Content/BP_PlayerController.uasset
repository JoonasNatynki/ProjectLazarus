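; Player controller that creates the WBP_HUDBase widget on BeginPlay and handles basic movement and look input for the possessed pawn.
; Enhanced Input actions push movement along the pawn's forward and right vectors, negated for backward and left.
; Vertical look pitches the pawn's CameraComponent directly with an unclamped local rotation, while horizontal look feeds scaled controller yaw input.
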(event `self.ReceiveBeginPlay`
  (bind _returnvalue (`|CreateWidget` "/Game/WBP_HUDBase.WBP_HUDBase_C" self))
  (`UserWidget.AddToViewport` _returnvalue 0))

(event `EnhancedInput|/Game/InputActions/ForwardInputAction`
  (params (ActionValue :type Boolean) (ElapsedSeconds :type "Float (double-precision)") (TriggeredSeconds :type "Float (double-precision)") (InputAction :type "InputAction Object Reference" :default "/Game/InputActions/ForwardInputAction.ForwardInputAction"))
  (bind _returnvalue (`self.K2_GetPawn`))
  ;[0 0.02083 0.002638] Basic movement inputs
  (:`Triggered`
    (`Pawn.AddMovementInput` _returnvalue (`self.GetActorForwardVector` _returnvalue) 1.0 false)))

(event `EnhancedInput|/Game/InputActions/BackwardInputAction`
  (params (ActionValue :type Boolean) (ElapsedSeconds :type "Float (double-precision)") (TriggeredSeconds :type "Float (double-precision)") (InputAction :type "InputAction Object Reference" :default "/Game/InputActions/BackwardInputAction.BackwardInputAction"))
  (bind _returnvalue (`self.K2_GetPawn`))
  ;[0 0.02083 0.002638] Basic movement inputs
  (:`Triggered`
    (`Pawn.AddMovementInput` _returnvalue (`KismetMathLibrary.NegateVector` (`self.GetActorForwardVector` _returnvalue)) 1.0 false)))

(event `EnhancedInput|/Game/InputActions/MoveLeft`
  (params (ActionValue :type Boolean) (ElapsedSeconds :type "Float (double-precision)") (TriggeredSeconds :type "Float (double-precision)") (InputAction :type "InputAction Object Reference" :default "/Game/InputActions/MoveLeft.MoveLeft"))
  (bind _returnvalue (`self.K2_GetPawn`))
  ;[0 0.02083 0.002638] Basic movement inputs
  (:`Triggered`
    (`Pawn.AddMovementInput` _returnvalue (`KismetMathLibrary.NegateVector` (`self.GetActorRightVector` _returnvalue)) 1.0 false)))

(event `EnhancedInput|/Game/InputActions/MoveRight`
  (params (ActionValue :type Boolean) (ElapsedSeconds :type "Float (double-precision)") (TriggeredSeconds :type "Float (double-precision)") (InputAction :type "InputAction Object Reference" :default "/Game/InputActions/MoveRight.MoveRight"))
  (bind _returnvalue (`self.K2_GetPawn`))
  ;[0 0.02083 0.002638] Basic movement inputs
  (:`Triggered`
    (`Pawn.AddMovementInput` _returnvalue (`self.GetActorRightVector` _returnvalue) 1.0 false)))

(event `EnhancedInput|/Game/InputActions/LookUpDown`
  (params (ActionValue :type "Float (double-precision)") (ElapsedSeconds :type "Float (double-precision)") (TriggeredSeconds :type "Float (double-precision)") (InputAction :type "InputAction Object Reference" :default "/Game/InputActions/LookUpDown.LookUpDown"))
  (bind _returnvalue (`self.GetComponentByClass` (`self.K2_GetPawn`) "/Script/Engine.CameraComponent"))
  ;[0 0.02083 0.002638] Basic camera inputs
  (:`Triggered`
    (`/Engine/EditorBlueprintResources/StandardMacros.IsValid` _returnvalue
      (:`Is Valid`
        (`SceneComponent.K2_AddLocalRotation` _returnvalue (`KismetMathLibrary.MakeRotator` 0.0 ActionValue) false false)))))

(event `EnhancedInput|/Game/InputActions/LookLeftRight`
  (params (ActionValue :type "Float (double-precision)") (ElapsedSeconds :type "Float (double-precision)") (TriggeredSeconds :type "Float (double-precision)") (InputAction :type "InputAction Object Reference" :default "/Game/InputActions/LookLeftRight.LookLeftRight"))
  ;[0 0.02083 0.002638] Basic camera inputs
  (:`Triggered`
    (`Pawn.AddControllerYawInput` (`self.K2_GetPawn`) (* ActionValue 0.35))))

(fn `UserConstructionScript`)